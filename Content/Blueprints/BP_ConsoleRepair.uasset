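; BP_ConsoleRepair is a repair table actor that displays a console's mesh alongside a repair widget.
; Initializing with console data, guarded by a check on current data, async-loads the mesh, then fills the widget and binds the salvage event.
; Salvage clears the table, hiding the mesh and resetting the widget to its empty state.
; The widget starts hidden and appears after a short delay when toggled on.
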(event `Toggle Repair Widget`
  (params (bNewVisibility :type Boolean))
  (if bNewVisibility
    (`KismetSystemLibrary.Delay` 0.2))
  (`SceneComponent.SetVisibility` (`self.Widget`) bNewVisibility false))

(event `self.ReceiveBeginPlay`
  (bind _asw_repair (cast `/Game/UI/Repair/W_Repair` (`WidgetComponent.GetUserWidgetObject` (`self.Widget`))))
  (set `self.RepairWidget` _asw_repair)
  (`SceneComponent.SetVisibility` (`self.ConsoleMesh`) false false)
  (`self.Toggle Repair Widget` false))

(event `Remove Console From Table`
  (set `self.In Console Data` null)
  (`SceneComponent.SetVisibility` (`self.ConsoleMesh`) false false)
  (`/Game/UI/Repair/W_Repair.Reset To Empty State` (`self.RepairWidget`)))

(event `Initialize With Console`
  (params (InConsoleData :type "/Game/Blueprints/Consoles/BP_ConsoleData Object Reference"))
  (bind _consolemesh (`self.ConsoleMesh`))
  (bind _in_console_data (`self.In Console Data`))
  (if (not (and (`KismetSystemLibrary.IsValid` _in_console_data) (!= _in_console_data InConsoleData)))
    (set `self.In Console Data` InConsoleData)
    (bind _object (`|LoadAsset` (`.Mesh_10_8C0CF5B34DC9C524A8E1BD810751D003` (break `/Game/Blueprints/Consoles/FConsoleInfo` (`/Game/Blueprints/Consoles/BP_ConsoleData.ConsoleInfo` InConsoleData))))
      (:`Completed`
        (bind _asstatic_mesh (cast `StaticMesh` _object))
        (`StaticMeshComponent.SetStaticMesh` _consolemesh _asstatic_mesh)
        (`SceneComponent.SetVisibility` _consolemesh true false)
        (`/Game/UI/Repair/W_Repair.Initialize WIth Console` (`self.RepairWidget`) (`self.In Console Data`))
        (add `/Game/Blueprints/Consoles/BP_ConsoleData.OnSalvage` InConsoleData (delegate `Handle Salvage`))
        (add `/Game/Blueprints/Consoles/BP_ConsoleData.OnSalvage` (`self.In Console Data`) (delegate `Handle Salvage`))))))

(event `Handle Salvage`
  (`self.Remove Console From Table`))

(fn `UserConstructionScript`)