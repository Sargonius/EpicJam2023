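; BP_QueueManager spawns customers and tracks how many are in the queue.
; SpawnCustomer creates a BP_Customer at the spawn point actor's transform, owned by the manager, and plays a new-customer sound while the count is below the maximum.
; NotifyOnExitQueue decrements the count, freeing room for later spawns.
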(event `Spawn Customer`
  (if (< (`self.CurrentCustomersInQueue`) (`self.MaxCustomersInQueue`))
    (`|SpawnActorFromClass` "/Game/Blueprints/Customers/BP_Customer.BP_Customer_C" (`self.GetTransform` (`self.SpawnPointActor`)) "AlwaysSpawn" "MultiplyWithRoot" self null)
    (`GameplayStatics.PlaySound2D` "/Game/Sound/S_NewCustomer_Cue.S_NewCustomer_Cue" 1.0 1.0 0.0 null null)
    (`/Engine/EditorBlueprintResources/StandardMacros.IncrementInt` (`self.CurrentCustomersInQueue`))))

(event `Notify On Exit Queue`
  (`/Engine/EditorBlueprintResources/StandardMacros.DecrementInt` (`self.CurrentCustomersInQueue`)))

(fn `UserConstructionScript`)