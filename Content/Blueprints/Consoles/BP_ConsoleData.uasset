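; BP_ConsoleData holds the state of one console, built from a ConsoleInfo passed in at initialization.
; GenerateBrokenParts copies and shuffles the info's part list, then flips a coin per part to split it into WorkingParts and BrokenParts, iterating in reverse so removal is safe.
; Salvage is a stub that loops over the working parts without acting on them.
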(event `Initialize With Console Info`
  (params (InConsoleInfo :type "/Game/Blueprints/Consoles/FConsoleInfo Structure"))
  (set `self.ConsoleInfo` InConsoleInfo))

(event `Generate Broken Parts`
  (bind _workingparts (`self.WorkingParts`))
  (bind _output_get (set `self.WorkingParts` (`.Parts_18_B0DA27854A72FBAB8BB882BE609BD244` (break `/Game/Blueprints/Consoles/FConsoleInfo` (`self.ConsoleInfo`)))))
  (`KismetArrayLibrary.Array_Shuffle` _output_get)
  (bind (_arrayindex _arrayelement) (`/Engine/EditorBlueprintResources/StandardMacros.ReverseForEachLoop` _workingparts)
    (:`LoopBody`
      ;[1 1 1] IsBroken
      (if (`KismetMathLibrary.RandomBool`)
        (`KismetArrayLibrary.Array_Add` (`self.BrokenParts`) _arrayelement)
        (`KismetArrayLibrary.Array_Remove` _workingparts _arrayindex)))))

(event `Salvage`
  (for _ (`self.WorkingParts`)
    _))