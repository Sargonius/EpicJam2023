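; BP_CameraManager switches the player's view between a store camera and a workbench camera.
; BeginPlay forces the store camera as the view target with no blend time specified.
; Two events, SwitchToStoreCamera and SwitchToWorkbenchCamera, blend to their camera over a short transition.
; Every switch goes through SetViewTargetWithBlend on the CSS player controller, with the outgoing view locked.
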(event `self.ReceiveBeginPlay`
  ;[1 1 1] Force Store Camera
  (`PlayerController.SetViewTargetWithBlend` (`/Game/Blueprints/BPFL_Game.GetCSSPlayerController`) (`self.StoreCamera`) 0.0 "VTBlend_Linear" 0.0 true))

(event `Switch To Store Camera`
  (`PlayerController.SetViewTargetWithBlend` (`/Game/Blueprints/BPFL_Game.GetCSSPlayerController`) (`self.StoreCamera`) 0.5 "VTBlend_Linear" 0.0 true))

(event `Switch To Workbench Camera`
  (`PlayerController.SetViewTargetWithBlend` (`/Game/Blueprints/BPFL_Game.GetCSSPlayerController`) (`self.WorkbenchCamera`) 0.5 "VTBlend_Linear" 0.0 true))

(fn `UserConstructionScript`)