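; Game state for a console repair-and-trade shop game, holding the day cycle, money, spare parts, upgrades and current player state.
; Timers advance game minutes and end the day, deferring closing until an active trade ends, then charge rent and show results or defeat.
; Inventory and money changes broadcast update events.
; It also toggles the repair widget by state, puts bought consoles into inventory and shows victory on a specific upgrade.
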(event `Start Minute Countdown`
  ;[1 1 1] Converting Game Hours to minute update timer
  (set `self.MinutesInGameDay` (* (- (`self.GameDayEndHour`) (`self.GameDayStartHour`)) 60))
  (bind _returnvalue (`KismetSystemLibrary.K2_SetTimerDelegate` (delegate `Update Game Time`) (/ (`self.DayDurationInRealSeconds`) (`self.MinutesInGameDay`)) true))
  (set `self.CurrentTimeUpdateHandle` _returnvalue))

(event `Update Game Time`
  ;[1 1 1] Will be converted to 10:30 in UI
  (`/Engine/EditorBlueprintResources/StandardMacros.IncrementInt` (`self.CurrentTimeInMinutes`)
    (:`  `
      (`self.OnTimeUpdate`))))

(event `Start Day Timer`
  (`KismetSystemLibrary.K2_SetTimerDelegate` (delegate `End Current Day`) (`self.DayDurationInRealSeconds`))
  (`self.Start Minute Countdown`)
  (`self.OnNewDay`)
  (set `self.DayProfit` 0))

(event `End Current Day`
  (bind _currentstate (`self.CurrentState`))
  ;[1 1 1] ... :D
  (`KismetSystemLibrary.K2_ClearAndInvalidateTimerHandle` (`self.CurrentTimeUpdateHandle`))
  (if (or (`|EnumEquality` _currentstate "NewEnumerator2") (`|EnumEquality` _currentstate "NewEnumerator3"))
    (add `self.OnTradeEnded` (delegate `Handle Delayed End of Day`))
    (else
      (`self.OnDayEnded` :!label _label)
      (if (`self.Has Money` (`self.RentPayment`))
        (`self.Consume Money` (`self.RentPayment`))
        (`/Engine/EditorBlueprintResources/StandardMacros.IncrementInt` (`self.CurrentDay`)
          (:`  `
            (set `self.CurrentTimeInMinutes` 0)
            (`self.OnTimeUpdate`)
            (bind _returnvalue (`|CreateWidget` "/Game/UI/Screens/W_Modal_DayResults.W_Modal_DayResults_C"))
            (`UserWidget.AddToViewport` _returnvalue 0)))
        (else
          (bind _returnvalue_2 (`|CreateWidget` "/Game/UI/Screens/W_Modal_Defeat.W_Modal_Defeat_C"))
          (`UserWidget.AddToViewport` _returnvalue_2 0))))))

(event `Handle Delayed End of Day`
  ;[1 1 1] ... :D
  (remove `self.OnTradeEnded` (delegate `Handle Delayed End of Day`))
  (goto _label))

(fn `Add Money`
  (params (Amount :type Integer))
  (set `self.CurrentMoney` (+ (`self.CurrentMoney`) Amount))
  (set `self.DayProfit` (+ (`self.DayProfit`) Amount))
  (`self.OnMoneyUpdate`))

(fn `Add Spare Part`
  (params (PartType :type "/Game/Blueprints/Consoles/EPartType Enum" :default "NewEnumerator0"))
  (locals (NewAmount :type Integer))
  (bind _spareparts (`self.SpareParts`))
  (bind (_value _returnvalue) (`BlueprintMapLibrary.Map_Find` _spareparts PartType))
  (if _returnvalue
    (bind _output_get (set `local.NewAmount` (+ _value 1)))
    (`BlueprintMapLibrary.Map_Add` (`self.SpareParts`) PartType _output_get)
    (`self.OnSparePartUpdate` "NewEnumerator0" (`local.NewAmount`))
    (else
      (set `local.NewAmount` 1)
      (`BlueprintMapLibrary.Map_Add` _spareparts PartType (`local.NewAmount`))
      (`self.OnSparePartUpdate` PartType (`local.NewAmount`)))))

(fn `Buy Console`
  (params (InConsoleInfo :type "/Game/Blueprints/Consoles/FConsoleInfo Structure"))
  (bind _returnvalue (`|GenericCreateObject` "/Game/Blueprints/Consoles/BP_ConsoleData.BP_ConsoleData_C"))
  (`/Game/Blueprints/Consoles/BP_ConsoleData.Initialize With Console Info` _returnvalue InConsoleInfo (`/Game/Blueprints/BPFL_Game.GetCSSGameState`))
  (`/Game/UI/Inventory/W_InventoryPanel.Put Console in First Free Slot` (`/Game/UI/Screens/W_GameHud.W_InventoryPanel` (`/Game/Blueprints/BPFL_Game.Get Hud`)) _returnvalue))

(fn `Consume Money`
  (params (Amount :type Integer))
  (if (`self.Has Money` Amount)
    (set `self.CurrentMoney` (- (`self.CurrentMoney`) Amount))
    (set `self.DayProfit` (- (`self.DayProfit`) Amount))
    (`self.OnMoneyUpdate`)))

(fn `Consume Spare Part`
  (params (PartType :type "/Game/Blueprints/Consoles/EPartType Enum" :default "NewEnumerator0"))
  (returns (bSuccess :type Boolean))
  (locals (NewAmount :type Integer))
  (bind _spareparts (`self.SpareParts`))
  (bind (_value _returnvalue) (`BlueprintMapLibrary.Map_Find` _spareparts PartType))
  (if _returnvalue
    (if (> _value 0)
      (bind _output_get (set `local.NewAmount` (- _value 1)))
      (`BlueprintMapLibrary.Map_Add` _spareparts PartType _output_get)
      (`self.OnSparePartUpdate` PartType (`local.NewAmount`))
      (return true)
      (else
        _)))
  (return false))

(fn `Has Money`
  (params (Amount :type Integer))
  (returns (bHas :type Boolean))
  (return (<= Amount (`self.CurrentMoney`))))

(fn `Has Spare Part`
  (params (PartType :type "/Game/Blueprints/Consoles/EPartType Enum" :default "NewEnumerator0"))
  (returns (bHas :type Boolean) (Amount :type Integer))
  (locals (NewAmount :type Integer))
  (bind (_value _returnvalue) (`BlueprintMapLibrary.Map_Find` (`self.SpareParts`) PartType))
  (if _returnvalue
    (return (> _value 0) _value)
    (else
      (return false 0))))

(fn `HasUpgrade`
  (params (InUpgrade :type "/Game/Blueprints/EUpgradeType Enum (by ref)"))
  (returns (bHasUpgrade :type Boolean))
  (return (`BlueprintMapLibrary.Map_Find` (`self.Upgrades`) InUpgrade)))

(fn `Set Current State`
  (params (CurrentState :type "/Game/Blueprints/ECurrentState Enum" :default "NewEnumerator0"))
  (bind _outrepairtable (`/Game/Blueprints/BPFL_Game.GetRepairTable`))
  (bind _output_get (set `self.CurrentState` CurrentState))
  (switch `/Game/Blueprints/ECurrentState` _output_get
    (:`NewEnumerator0`
      (`/Game/Blueprints/BP_ConsoleRepair.Toggle Repair Widget` _outrepairtable false :!label _label))
    (:`NewEnumerator1`
      (`/Game/Blueprints/BP_ConsoleRepair.Toggle Repair Widget` _outrepairtable true))
    (:`NewEnumerator2`
      (goto _label))))

(fn `UnlockUpgrade`
  (params (InUpgrade :type "/Game/Blueprints/EUpgradeType Enum (by ref)"))
  (`BlueprintMapLibrary.Map_Add` (`self.Upgrades`) InUpgrade true)
  (if (`|EnumEquality` InUpgrade (enumliteral `/Game/Blueprints/EUpgradeType` "NewEnumerator4"))
    (bind _returnvalue (`|CreateWidget` "/Game/UI/Screens/W_Modal_Victory.W_Modal_Victory_C"))
    (`UserWidget.AddToViewport` _returnvalue 0)))

(fn `UserConstructionScript`)