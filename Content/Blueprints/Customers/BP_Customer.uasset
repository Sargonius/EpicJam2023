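; BP_Customer is an AI shop customer that wants a random console from DT_Consoles, with budget scaled by random difficulty.
; It claims the single queue spot, or wanders and retries while occupied.
; A looping timer drains upgrade-scalable patience shown in its info widget, and stops when trade starts.
; Expired patience or trade end sends it to an exit point, where it destroys itself and notifies BP_QueueManager.
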(event `Start Trade`
  (`KismetSystemLibrary.K2_ClearAndInvalidateTimerHandle` (`self.PatienceHandler`))
  (`SceneComponent.SetVisibility` (`self.CustomerInfoUI`) false false))

(event `self.ReceiveBeginPlay`
  (bind _queuespot (`self.QueueSpot`))
  (set `self.Difficulty` (`KismetArrayLibrary.Array_Random` (`|MakeArray` "NewEnumerator0" "NewEnumerator1" "NewEnumerator2" :!type "/Game/Blueprints/EDifficulty Enum")))
  (add `/Game/Blueprints/BP_CSSGameState.OnDayEnded` (`/Game/Blueprints/BPFL_Game.GetCSSGameState`) (`|CreateDelegate` :!event `Quit Queue`))
  (`self.Generate Customer Request`)
  (bind _outactors (`GameplayStatics.GetAllActorsOfClass` "/Game/Blueprints/BP_QueueSpot.BP_QueueSpot_C"))
  (set `self.QueueSpot` (`|GetArrayItem` _outactors))
  (bind _returnvalue (`KismetSystemLibrary.K2_SetTimerDelegate` (delegate `Tick Patience`) 1.0 true))
  (set `self.PatienceHandler` _returnvalue)
  (`self.Initialize Customer UI`)
  (if (`/Game/Blueprints/BP_QueueSpot.bIsOccupied` _queuespot) :!label _label
    (`AITask_MoveTo.AIMoveTo` (`AIBlueprintHelperLibrary.GetAIController` self) (`NavigationSystemV1.K2_GetRandomReachablePointInRadius` (`self.K2_GetActorLocation`) 1500.0 null null) null
      (:`OnMoveFinished`
        (`self.Try To Get To The Counter`)))
    (else
      (set `self.bIsActiveCustomer` true)
      (set `/Game/Blueprints/BP_QueueSpot.bIsOccupied` true _queuespot)
      (`AITask_MoveTo.AIMoveTo` (`AIBlueprintHelperLibrary.GetAIController` self) (0.0 0.0 0.0) _queuespot
        (:`then`
          (add `/Game/Blueprints/BP_CSSGameState.OnTradeEnded` (`/Game/Blueprints/BPFL_Game.GetCSSGameState`) (delegate `Handle Trade Ended`)))))))

(event `Try To Get To The Counter`
  (goto _label))

(event `Handle Trade Ended`
  (`self.Quit Queue`)
  (remove `/Game/Blueprints/BP_CSSGameState.OnTradeEnded` (`/Game/Blueprints/BPFL_Game.GetCSSGameState`) (delegate `Handle Trade Ended`)))

(event `Tick Patience`
  ;[1 1 1] Customer Patience
  (`/Engine/EditorBlueprintResources/StandardMacros.DecrementFloat` (`self.Patience`)
    (:`  `
      (`self.OnPatienceUpdated`)
      (if (<= (`self.Patience`) 0.0)
        (`KismetSystemLibrary.K2_ClearAndInvalidateTimerHandle` (`self.PatienceHandler`))
        (`self.Quit Queue`)))))

(event `Quit Queue`
  ;[1 1 1] Quit Queue
  (if (`self.bIsActiveCustomer`)
    (`/Game/Blueprints/BP_QueueSpot.Change Occupation Status` (`self.QueueSpot`) false))
  (bind _outactors (`GameplayStatics.GetAllActorsOfClass` "/Game/Blueprints/Customers/BP_ExitPoint.BP_ExitPoint_C"))
  (`AITask_MoveTo.AIMoveTo` (`AIBlueprintHelperLibrary.GetAIController` self) (0.0 0.0 0.0) (`|GetArrayItem` _outactors)
    (:`then`
      (`SceneComponent.SetVisibility` (`self.CustomerInfoUI`) false false))
    (:`OnRequestFailed`
      (`self.K2_DestroyActor` :!label _label_2)
      (bind _outactors_2 (`GameplayStatics.GetAllActorsOfClass` "/Game/Blueprints/BP_QueueManager.BP_QueueManager_C"))
      (`/Game/Blueprints/BP_QueueManager.Notify On Exit Queue` (`|GetArrayItem` _outactors_2)))
    (:`OnMoveFinished`
      (goto _label_2))))

(fn `Generate Customer Request`
  (bind _outrownames (`DataTableFunctionLibrary.GetDataTableRowNames` "/Game/Blueprints/Consoles/DT_Consoles.DT_Consoles"))
  (bind _returnvalue (`|GetDataTableRow` "/Game/Blueprints/Consoles/DT_Consoles.DT_Consoles" (`KismetArrayLibrary.Array_Random` _outrownames))
    (:`then`
      (bind _output_get (set `self.RequiredItem` _returnvalue))
      (bind (_id _name _icon _mesh _baseprice) (break `/Game/Blueprints/Consoles/FConsoleInfo` _output_get))
      (set `self.Money` (select `/Game/Blueprints/EDifficulty` (`self.Difficulty`) :`NewEnumerator0` (* _baseprice 2) :`NewEnumerator1` _baseprice :`NewEnumerator2` (`KismetMathLibrary.FTrunc` (* (`KismetMathLibrary.Conv_IntToDouble` _baseprice) 0.8))))
      (bind _output_get_2 (set `self.MaxPatience` (* (`KismetMathLibrary.RandomFloatInRange` 30.0 60.0) (`KismetMathLibrary.SelectFloat` 2.0 1.0 (`/Game/Blueprints/BPFL_Game.HasUpgrade` "NewEnumerator2")))))
      (set `self.Patience` _output_get_2))))

(fn `GetPatienceFillPercentForUI`
  (returns (OutFillPercent :type "Float (double-precision)"))
  (return (`KismetMathLibrary.MapRangeClamped` (`self.Patience`) 0.0 (`self.MaxPatience`) 1.0)))

(fn `IncreasePatience`
  (set `self.Patience` (+ (`self.Patience`) 1.0))
  (set `self.MaxPatience` (+ (`self.MaxPatience`) 1.0))
  (`self.OnPatienceUpdated`))

(fn `Initialize Customer UI`
  (bind _asw_customer_info (cast `/Game/UI/Customer/W_CustomerInfo` (`WidgetComponent.GetUserWidgetObject` (`self.CustomerInfoUI`))))
  (`/Game/UI/Customer/W_CustomerInfo.Initialize With Customer` _asw_customer_info self))

(fn `UserConstructionScript`)