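; Blueprint function library of global getters for core CSS game objects: the HUD, player controller, game mode and camera manager.
; The HUD and controller getters cast player controller 0 to BP_CSSPlayerController, and the HUD getter prints an error when the HUD is invalid.
; The camera manager getter searches all BP_CameraManager actors on every call and returns the first, without caching or a validity check.
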(fn `Get Hud`
  (returns (HUD :type "/Game/UI/Screens/W_GameHud Object Reference"))
  (bind _asbp_cssplayer_controller (cast `/Game/Blueprints/BP_CSSPlayerController` (`GameplayStatics.GetPlayerController` (`local.__WorldContext`))))
  (bind _hud (`/Game/Blueprints/BP_CSSPlayerController.HUD` _asbp_cssplayer_controller))
  (`/Engine/EditorBlueprintResources/StandardMacros.IsValid` _hud
    (:`Is Valid`
      (return _hud))
    (:`Is Not Valid`
      (`KismetSystemLibrary.PrintString` (`local.__WorldContext`) "ERROR: HUD is invalid"))))

(fn `GetCameraManager`
  (returns (`Camera Manager` :type "/Game/Blueprints/BP_CameraManager Object Reference"))
  ;[1 1 1] Lazy Getter
  (bind _outactors (`GameplayStatics.GetAllActorsOfClass` (`local.__WorldContext`) "/Game/Blueprints/BP_CameraManager.BP_CameraManager_C"))
  (return (`|GetArrayItem` _outactors)))

(fn `GetCSSGameMode`
  (returns (`BP CSSGame Mode` :type "/Game/Blueprints/BP_CSSGameMode Object Reference"))
  (bind _asbp_cssgame_mode (cast `/Game/Blueprints/BP_CSSGameMode` (`GameplayStatics.GetGameMode` (`local.__WorldContext`))))
  (return _asbp_cssgame_mode))

(fn `GetCSSPlayerController`
  (returns (`BP CSSPlayer Controller` :type "/Game/Blueprints/BP_CSSPlayerController Object Reference"))
  (bind _asbp_cssplayer_controller (cast `/Game/Blueprints/BP_CSSPlayerController` (`GameplayStatics.GetPlayerController` (`local.__WorldContext`))))
  (return _asbp_cssplayer_controller))